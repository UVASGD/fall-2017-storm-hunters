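; Drivable Mercedes vehicle pawn with first/third-person cameras, RepNotify lights, water-triggered engine stalling and a debug stats widget.
; Input goes through Server events to vehicle movement, with curve-based steering feeding the anim blueprint.
; Tick applies downforce, anti-drift and anti-roll forces, and detects per-wheel drifting to drive skid effects and tire audio alongside RPM-based engine sound.
; Exiting spawns and possesses a physics pawn, ragdolled at high speed.
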(event `self.Mesh.OnComponentBeginOverlap`
  (params (OverlappedComponent :type "PrimitiveComponent Object Reference") (OtherActor :type "Actor Object Reference") (OtherComp :type "PrimitiveComponent Object Reference") (OtherBodyIndex :type Integer) (bFromSweep :type Boolean) (SweepResult :type "HitResult Structure (by ref)"))
  ;[1 1 1] Flood Engine on Water Overlap
  (cast `/Game/Environment/BP_Water_Volume` OtherActor)
  (`self.Drowning Timer`)
  (goto _label :!via `Open`))

(event `self.Mesh.OnComponentEndOverlap`
  (params (OverlappedComponent :type "PrimitiveComponent Object Reference") (OtherActor :type "Actor Object Reference") (OtherComp :type "PrimitiveComponent Object Reference") (OtherBodyIndex :type Integer))
  ;[1 1 1] Flood Engine on Water Overlap
  (cast `/Game/Environment/BP_Water_Volume` OtherActor)
  (goto _label :!via `Close`))

(event `self.ReceivePossessed`
  (params (NewController :type "Controller Object Reference"))
  ;[1 1 1] Possession
  (`self.PossessPVehicle` NewController)
  (`KismetSystemLibrary.Delay` 1.0)
  (if (and (`self.RaceStarted`) (`self.InRace`))
    (set `self.Engine Started` true)))

(event `Drowning Timer`
  ;[1 1 1] Flood Engine on Water Overlap
  (`KismetSystemLibrary.Delay` 3.0)
  (`/Engine/EditorBlueprintResources/StandardMacros.Gate` true :!label _label
    (:`Exit`
      (`self.Stall Engine`)
      (set `self.Engine Drowned` true))))

(event `self.ReceiveBeginPlay`
  ;[1 1 1] Begin/End Play
  (`WidgetBlueprintLibrary.SetInputMode_GameOnly` (`GameplayStatics.GetPlayerController` 0))
  (`self.ActivatePCamera`)
  (`self.InitializeVehicle`))

(event `self.ReceiveEndPlay`
  (params (EndPlayReason :type "EEndPlayReason Enum" :default "Destroyed"))
  ;[1 1 1] Begin/End Play
)

(event `InputAction|Vehicle_LookBack`
  (params (Key :type "Key Structure"))
  ;[1 1 1] Local Inputs
  (:`Pressed`
    (set `self.Look Back` true))
  (:`Released`
    (set `self.Look Back` false)))

(event `InputAxis|Steer`
  (params (AxisValue :type "Float (single-precision)"))
  ;[1 1 1] Network Inputs
  (`self.Server Steering` AxisValue))

(event `Server Tick`
  ;[1 1 1] Update Functions
  (`self.Driver Helping Force`)
  (`self.Calculate Mileage`)
  (`self.Calculate Speed`)
  (`self.Detect Drifting`)
  (`self.Update Vehicle Sounds`))

(event `InputAxis|Vehicle_Throttle`
  (params (AxisValue :type "Float (single-precision)"))
  ;[1 1 1] Network Inputs
  (`self.Server Throttle` AxisValue))

(event `InputAction|Gear_Up`
  (params (Key :type "Key Structure"))
  (bind _vehiclemovement (`self.VehicleMovement`))
  ;[1 1 1] Local Inputs
  (:`Pressed`
    (`WheeledVehicleMovementComponent.SetTargetGear` _vehiclemovement (+ (`WheeledVehicleMovementComponent.GetCurrentGear` _vehiclemovement) 1) (not (`WheeledVehicleMovementComponent.GetUseAutoGears` _vehiclemovement)))))

(event `self.ReceiveTick`
  (params (DeltaSeconds :type "Float (single-precision)"))
  ;[1 1 1] Update Functions
  (`self.Look Around` (`self.GetInputAxisValue`) (`self.GetInputAxisValue`) DeltaSeconds)
  (`self.Server Tick`))

(event `InputAction|Gear_Down`
  (params (Key :type "Key Structure"))
  (bind _vehiclemovement (`self.VehicleMovement`))
  ;[1 1 1] Local Inputs
  (:`Pressed`
    (`WheeledVehicleMovementComponent.SetTargetGear` _vehiclemovement (+ (`WheeledVehicleMovementComponent.GetCurrentGear` _vehiclemovement) -1) (not (`WheeledVehicleMovementComponent.GetUseAutoGears` _vehiclemovement)))))

(event `InputAction|Handbrake`
  (params (Key :type "Key Structure"))
  ;[1 1 1] Network Inputs
  (:`Pressed`
    (`self.Server Handbrake` true))
  (:`Released`
    (`self.Server Handbrake` false)))

(event `InputAxis|Nitrous`
  (params (AxisValue :type "Float (single-precision)")))

(event `InputAction|ChangeView`
  (params (Key :type "Key Structure"))
  ;[1 1 1] Local Inputs
  (:`Pressed`
    (`self.Change Camera View`)))

(event `InputAction|Interact`
  (params (Key :type "Key Structure"))
  ;[1 1 1] Network Inputs
  (:`Pressed`
    (`self.Server Exit Vehicle`)))

(event `Key|Tab`
  (params (Key :type "Key Structure"))
  ;[1 1 1] Local Inputs
  (:`Pressed`
    (`/Engine/EditorBlueprintResources/StandardMacros.FlipFlop`
      (:`A`
        (`self.Debug Stats Widget` true))
      (:`B`
        (`self.Debug Stats Widget` false)))))

(event `InputAction|Vehicle_Lights`
  (params (Key :type "Key Structure"))
  ;[1 1 1] Network Inputs
  (:`Pressed`
    (`self.Server Headlight`)))

(event `Server Exit Vehicle`
  ;[1 1 1] Server Events
  (`self.UnPossessPVehicle`))

(event `Server Steering`
  (params (`Axis Value` :type "Float (double-precision)"))
  ;[1 1 1] Server Events
  (`self.Set Steering Angle` `Axis Value`)
  (set `/Game/Vehicles/Mercedes/Mercedes_Anim_BP.Steering Angle` (`self.Steering Angle Calc`) (`self.Vehicle Anim BP`))
  (`WheeledVehicleMovementComponent.SetSteeringInput` (`self.VehicleMovement`) `Axis Value`))

(event `Server Throttle`
  (params (`Axis Value` :type "Float (double-precision)"))
  (bind _returnvalue (< `Axis Value` 0.0))
  ;[1 1 1] Server Events
  (if (`self.Engine Started`)
    (set `self.Is Braking` (and (> (`WheeledVehicleMovementComponent.GetForwardSpeed` (`self.VehicleMovement`)) 0.0) _returnvalue))
    (set `self.Is Reversing` (and _returnvalue (== (`WheeledVehicleMovementComponent.GetCurrentGear` (`self.VehicleMovement`)) -1)))
    (`WheeledVehicleMovementComponent.SetThrottleInput` (`self.VehicleMovement`) `Axis Value`)
    (else
      (`WheeledVehicleMovementComponent.SetThrottleInput` (`self.VehicleMovement`) 0.0))))

(event `Server Handbrake`
  (params (`Apply Handbrake` :type Boolean))
  ;[1 1 1] Server Events
  (`WheeledVehicleMovementComponent.SetHandbrakeInput` (`self.VehicleMovement`) `Apply Handbrake`))

(event `Server Headlight`
  ;[1 1 1] Server Events
  (`self.Toggle Headlights`))

(fn `ActivatePCamera`
  (bind _is_third_person_view (`self.Is Third Person View`))
  (`ActorComponent.SetActive` (`self.TP_Camera`) _is_third_person_view false)
  (`ActorComponent.SetActive` (`self.FP_Camera`) (not _is_third_person_view) false))

(fn `Calculate Mileage`
  (set `self.Mileage` (+ (`self.Mileage`) (* (/ (`KismetMathLibrary.Abs` (`self.Speed`)) 3600.0) (`GameplayStatics.GetWorldDeltaSeconds`)))))

(fn `Calculate Speed`
  (locals (`Temp Speed` :type "Float (double-precision)"))
  (set `self.Speed` (`WheeledVehicleMovementComponent.GetForwardSpeed` (`self.VehicleMovement`)))
  (set `self.RPM` (`WheeledVehicleMovementComponent.GetEngineRotationSpeed` (`self.VehicleMovement`))))

(fn `Camera Distance`
  (bind _tp_springarm (`self.TP_SpringArm`))
  (bind _fp_camera (`self.FP_Camera`))
  (bind (_relativelocation_x _relativelocation_y _relativelocation_z) (`KismetMathLibrary.BreakVector` (`SceneComponent.RelativeLocation` _tp_springarm)))
  (bind (_relativelocation_x_2 _relativelocation_y_2 _relativelocation_z_2) (`KismetMathLibrary.BreakVector` (`SceneComponent.RelativeLocation` _fp_camera)))
  ;[1 1 1] Third Person
  (`SceneComponent.K2_SetRelativeLocation` _tp_springarm (`KismetMathLibrary.MakeVector` (`KismetMathLibrary.MapRangeClamped` (* (`KismetMathLibrary.VSize` (`self.GetVelocity`)) 0.036) -90.0 90.0 150.0 -150.0) _relativelocation_y _relativelocation_z) false false)
  ;[1 1 1] First Person
  (`SceneComponent.K2_SetRelativeLocation` _fp_camera (`KismetMathLibrary.MakeVector` (`KismetMathLibrary.MapRangeClamped` (* (`KismetMathLibrary.VSize` (`self.GetVelocity`)) 0.036) -20.0 20.0 10.0 -10.0) _relativelocation_y_2 _relativelocation_z_2) false false))

(fn `Change Camera View`
  (if (`self.Can Change View`)
    (bind _output_get (set `self.Is Third Person View` (not (`self.Is Third Person View`))))
    (`ActorComponent.SetActive` (`self.TP_Camera`) _output_get false)
    (`ActorComponent.SetActive` (`self.FP_Camera`) (not _output_get) false)))

(fn `Debug Stats Widget`
  (params (Show :type Boolean))
  (bind _returnvalue (`GameplayStatics.GetPlayerController` 0))
  (bind _returnvalue_2 (`GameplayStatics.GetPlayerController` 0))
  (bind _debug_widget (`self.Debug Widget`))
  (if Show
    (if (not (`KismetSystemLibrary.IsValid` (`self.Debug Widget`)))
      (bind _returnvalue_3 (`|CreateWidget` "/Game/UMG/Vehicle_Stats_Debug.Vehicle_Stats_Debug_C"))
      (bind _output_get (set `self.Debug Widget` _returnvalue_3))
      (set `/Game/UMG/Vehicle_Stats_Debug.Target Vehicle` self _output_get))
    (`UserWidget.AddToViewport` _output_get 1)
    (set `PlayerController.bShowMouseCursor` true _returnvalue_2)
    (`WidgetBlueprintLibrary.SetInputMode_GameAndUIEx` _returnvalue_2 (`self.Debug Widget`))
    (else
      (`/Engine/EditorBlueprintResources/StandardMacros.IsValid` _debug_widget
        (:`Is Valid`
          (`Widget.RemoveFromParent` _debug_widget)
          (set `PlayerController.bShowMouseCursor` false _returnvalue)
          (`WidgetBlueprintLibrary.SetInputMode_GameOnly` _returnvalue))))))

(fn `Detect Drifting`
  (bind _mesh (`self.Mesh`))
  (bind _mesh_2 (`self.Mesh`))
  (bind _mesh_3 (`self.Mesh`))
  (bind _mesh_4 (`self.Mesh`))
  (bind _mesh_5 (`self.Mesh`))
  (bind (_returnvalue_roll _returnvalue_pitch _returnvalue_yaw) (`KismetMathLibrary.BreakRotator` (`SceneComponent.K2_GetComponentRotation` _mesh_4)))
  (bind (_returnvalue_roll_2 _returnvalue_pitch_2 _returnvalue_yaw_2) (`KismetMathLibrary.BreakRotator` (`KismetMathLibrary.Conv_VectorToRotator` (`SceneComponent.GetComponentVelocity` _mesh_5))))
  (bind (_returnvalue_roll_3 _returnvalue_pitch_3 _returnvalue_yaw_3) (`KismetMathLibrary.BreakRotator` (`KismetMathLibrary.Conv_VectorToRotator` (`SceneComponent.GetComponentVelocity` _mesh_3))))
  (for (_array_element _array_index) (`self.Wheels`)
    (bind (_bonename _radius _steeringangle _mirrorsteering _applytorque _brakestrengthmultiplier _applyhandbrake _isonground _isdrifting) (break `/Game/Vehicles/00_Master_Vehicle/Structs/Wheel_Structure` _array_element))
    (bind _returnvalue (`PrimitiveComponent.GetPhysicsLinearVelocity` _mesh_2 _bonename))
    (bind _returnvalue_2 (`PrimitiveComponent.GetPhysicsAngularVelocity` _mesh _bonename))
    (bind (_returnvalue_x _returnvalue_y) (`KismetMathLibrary.BreakVector` (`KismetMathLibrary.InverseTransformDirection` (`SceneComponent.GetSocketTransform` _mesh _bonename "RTS_World") _returnvalue_2)))
    (bind (_returnvalue_x_2 _returnvalue_y_2 _returnvalue_z) (`KismetMathLibrary.BreakVector` (`KismetMathLibrary.InverseTransformDirection` (`SceneComponent.GetSocketTransform` _mesh_2 "None" "RTS_World") _returnvalue)))
    (bind _returnvalue_3 (`KismetMathLibrary.VSize` (`KismetMathLibrary.MakeVector` _returnvalue_x_2 0.0 _returnvalue_z)))
    (if (and (or (> (`KismetMathLibrary.Abs` (/ (* (* (`KismetMathLibrary.DegreesToRadians` _returnvalue_y) _radius) 0.036) (* _returnvalue_3 0.036))) 4.0) (> (`KismetMathLibrary.Abs` _returnvalue_y_2) 500.0)) _isonground (> (`KismetMathLibrary.VSize` (`KismetMathLibrary.MakeVector` _returnvalue_3 _returnvalue_y_2)) 700.0))
      (bind (_bonename_2 _radius_2) (break `/Game/Vehicles/00_Master_Vehicle/Structs/Wheel_Structure` _array_element))
      (`GameplayStatics.SpawnEmitterAtLocation` "/Game/Vehicles/00_Master_Vehicle/Effects/Smoke/PS_Smoke.PS_Smoke" (- (`SceneComponent.GetSocketLocation` _mesh_4 _bonename_2) (`KismetMathLibrary.MakeVector` 0.0 0.0 _radius_2)) (`KismetMathLibrary.MakeRotator` 0.0 0.0 _returnvalue_yaw))
      (if _isdrifting
        (bind (_bonename_3 _radius_3 _steeringangle_2 _mirrorsteering_2 _applytorque_2 _brakestrengthmultiplier_2 _applyhandbrake_2 _isonground_2 _isdrifting_2 _skidemitter) (break `/Game/Vehicles/00_Master_Vehicle/Structs/Wheel_Structure` _array_element))
        (`SceneComponent.K2_SetWorldTransform` _skidemitter (`KismetMathLibrary.MakeTransform` (- (`SceneComponent.GetSocketLocation` _mesh_3 _bonename_3) (`KismetMathLibrary.MakeVector` 0.0 0.0 (- _radius_3 2.0))) (`KismetMathLibrary.MakeRotator` 90.0 0.0 _returnvalue_yaw_3)) false false)
        (else
          (bind (_bonename_4 _radius_4) (break `/Game/Vehicles/00_Master_Vehicle/Structs/Wheel_Structure` _array_element))
          (bind _returnvalue_4 (`GameplayStatics.SpawnEmitterAtLocation` "/Game/Vehicles/00_Master_Vehicle/Effects/Skid/PS_Skid.PS_Skid" (- (`SceneComponent.GetSocketLocation` _mesh_5 _bonename_4) (`KismetMathLibrary.MakeVector` 0.0 0.0 (- _radius_4 2.0))) (`KismetMathLibrary.MakeRotator` 90.0 0.0 _returnvalue_yaw_2) false))
          (bind _structout (setmembers `/Game/Vehicles/00_Master_Vehicle/Structs/Wheel_Structure` :`StructRef` _array_element :`Is Drifting` true :`Skid Emitter` _returnvalue_4))
          (`KismetArrayLibrary.Array_Set` (`self.Wheels`) _array_index _structout)))
      (elif _isdrifting
        (bind _structout_2 (setmembers `/Game/Vehicles/00_Master_Vehicle/Structs/Wheel_Structure` :`StructRef` _array_element :`Is Drifting` false))
        (`KismetArrayLibrary.Array_Set` (`self.Wheels`) _array_index _structout_2)
        (`ActorComponent.Deactivate` (`.SkidEmitter_44_BE1B6F9348BF2F6C7397289CAA4F573E` (break `/Game/Vehicles/00_Master_Vehicle/Structs/Wheel_Structure` _array_element)))))))

(fn `Driver Helping Force`
  (bind _mesh (`self.Mesh`))
  (bind _mesh_2 (`self.Mesh`))
  (bind _wheels (`self.Wheels`))
  (bind _wheels_2 (`self.Wheels`))
  (bind _mesh_3 (`self.Mesh`))
  (bind _returnvalue (`SceneComponent.K2_GetComponentToWorld` _mesh_2))
  (bind _returnvalue_2 (`SceneComponent.K2_GetComponentToWorld` _mesh_3))
  (bind _output (`|GetArrayItem` (`SceneComponent.GetAllSocketNames` _mesh_3)))
  (`PrimitiveComponent.AddForce` (`self.Mesh`) (`KismetMathLibrary.MakeVector` 0.0 0.0 (* (`KismetMathLibrary.Abs` (`self.Additional Gravity Factor`)) -1.0)) "None" true)
  (if (`self.IsControlled`)
    ;[1 1 1] Wheels on Ground
    (bind _outactors (`GameplayStatics.GetAllActorsOfClass` "/Game/Weather/Tornado/Tornado_Pawn_BP.Tornado_Pawn_BP_C"))
    (for (_array_element _array_index) _wheels
      (bind (_bonename _radius) (break `/Game/Vehicles/00_Master_Vehicle/Structs/Wheel_Structure` _array_element))
      (bind _returnvalue_3 (`SceneComponent.GetSocketLocation` _mesh _bonename))
      (bind (_outhit _returnvalue_4) (`KismetSystemLibrary.LineTraceSingle` _returnvalue_3 (+ _returnvalue_3 (* (`SceneComponent.GetUpVector` _mesh) (* (+ _radius 1.0) -1.0))) "TraceTypeQuery1" false _outactors "None" true (struct :`R` 1.0 :`A` 1.0) (struct :`G` 1.0 :`A` 1.0) 0.1))
      (if _returnvalue_4
        (bind _structout (setmembers `/Game/Vehicles/00_Master_Vehicle/Structs/Wheel_Structure` :`StructRef` _array_element :`Is on Ground` true))
        (`KismetArrayLibrary.Array_Set` _wheels_2 _array_index _structout)
        ;[1 1 1] Antidrift Force
        (bind _returnvalue_5 (`PrimitiveComponent.GetPhysicsLinearVelocity` _mesh_2 _bonename))
        (bind (_returnvalue_x _returnvalue_y) (`KismetMathLibrary.BreakVector` (`KismetMathLibrary.InverseTransformDirection` _returnvalue _returnvalue_5)))
        (`PrimitiveComponent.SetPhysicsLinearVelocity` (`self.Mesh`) (`KismetMathLibrary.TransformDirection` _returnvalue (`KismetMathLibrary.MakeVector` 0.0 (* _returnvalue_y -1.0 (/ (`self.Anti-Drift Multiplier`) (`KismetMathLibrary.Conv_IntToDouble` (`KismetArrayLibrary.Array_Length` _wheels)))))) true "None")
        ;[1 1 1] Anti-Roll
        (bind _returnvalue_6 (`PrimitiveComponent.GetPhysicsAngularVelocity` _mesh_3 _output))
        (bind _returnvalue_x_2 (`KismetMathLibrary.BreakVector` (`KismetMathLibrary.InverseTransformDirection` _returnvalue_2 _returnvalue_6)))
        (`PrimitiveComponent.SetPhysicsAngularVelocity` (`self.Mesh`) (`KismetMathLibrary.TransformDirection` _returnvalue_2 (`KismetMathLibrary.MakeVector` (* _returnvalue_x_2 -1.0 (`self.Anti-Roll Multiplier`)))) true _output)
        (else
          (bind _structout_2 (setmembers `/Game/Vehicles/00_Master_Vehicle/Structs/Wheel_Structure` :`StructRef` _array_element :`Is on Ground` false))
          (`KismetArrayLibrary.Array_Set` _wheels_2 _array_index _structout_2))))))

(fn `InitializeVehicle`
  (bind _brake_light_material_slot_name (`self.Brake Light Material Slot Name`))
  (bind _mesh (`self.Mesh`))
  (set `self.Is Braking` false)
  (set `self.Is Head Light On` false)
  (if (not (== _brake_light_material_slot_name "None"))
    (bind _returnvalue (`PrimitiveComponent.CreateDynamicMaterialInstance` _mesh (`MeshComponent.GetMaterialIndex` _mesh _brake_light_material_slot_name) "/Game/Vehicles/00_Master_Vehicle/Materials/Instances/MI_BrakeLight.MI_BrakeLight"))
    (set `self.M Brake Light` _returnvalue)
    (bind _asmercedes_anim_bp (cast `/Game/Vehicles/Mercedes/Mercedes_Anim_BP` (`SkeletalMeshComponent.GetAnimInstance` (`self.Mesh`))))
    (set `self.Vehicle Anim BP` _asmercedes_anim_bp)))

(fn `Look Around`
  (params (LookUp :type "Float (double-precision)") (LookRight :type "Float (double-precision)") (DeltaTime :type "Float (double-precision)"))
  (bind _tp_springarm (`self.TP_SpringArm`))
  (bind _fp_camera (`self.FP_Camera`))
  (bind _fp_springarm (`self.FP_SpringArm`))
  (bind _returnvalue (`KismetMathLibrary.MakeRotator` 0.0 (* LookUp -1.0) LookRight))
  (bind (_relativerotation_roll _relativerotation_pitch _relativerotation_yaw) (`KismetMathLibrary.BreakRotator` (`SceneComponent.RelativeRotation` _fp_springarm)))
  (bind (_relativelocation_x _relativelocation_y _relativelocation_z) (`KismetMathLibrary.BreakVector` (`SceneComponent.RelativeLocation` _fp_camera)))
  (bind _relativerotation_roll_2 (`KismetMathLibrary.BreakRotator` (`SceneComponent.RelativeRotation` (`self.TP_SpringArm`))))
  (bind (_relativerotation_roll_3 _relativerotation_pitch_2 _relativerotation_yaw_2) (`KismetMathLibrary.BreakRotator` (`SceneComponent.RelativeRotation` _tp_springarm)))
  (bind (_returnvalue_roll _returnvalue_pitch _returnvalue_yaw) (`KismetMathLibrary.BreakRotator` (`KismetMathLibrary.SelectRotator` (`KismetMathLibrary.SelectRotator` (struct :`Pitch` -10.0 :`Yaw` 180.0) (struct :`Pitch` -10.0) (`self.Look Back`)) (`KismetMathLibrary.MakeRotator` 0.0 (`KismetMathLibrary.FClamp` _relativerotation_pitch_2 -50.0 10.0) _relativerotation_yaw_2) (`self.Auto rotate camera`))))
  (if (`self.Is Third Person View`)
    ;[1 1 1] Third Person Camera
    (if (`self.Auto Rotate Camera`)
      (`SceneComponent.K2_SetRelativeRotation` _tp_springarm (`KismetMathLibrary.MakeRotator` _relativerotation_roll_2 _returnvalue_pitch _returnvalue_yaw) false false)
      (`SceneComponent.K2_AddRelativeRotation` _tp_springarm (* _returnvalue 20.0) false false)
      (else
        (`SceneComponent.K2_AddRelativeRotation` _tp_springarm _returnvalue false false)))
    (else
      ;[1 1 1] First Person Camera
      (if (not (and (== LookUp 0.0) (== LookRight 0.0)))
        (`SceneComponent.K2_SetRelativeRotation` _fp_springarm (`KismetMathLibrary.MakeRotator` 0.0 (`KismetMathLibrary.FClamp` (+ _relativerotation_pitch (* LookUp 1.0)) -40.0 10.0) (`KismetMathLibrary.FClamp` (+ _relativerotation_yaw (* LookRight 1.0)) -110.0 160.0)) false false)
        (`SceneComponent.K2_SetRelativeLocation` _fp_camera (`KismetMathLibrary.MakeVector` _relativelocation_x (`KismetMathLibrary.MapRangeClamped` _relativerotation_yaw 70.0 160.0 0.0 -25.0) _relativelocation_z) false false)))))

(fn `OnRep_Is Braking`
  (bind _m_brake_light (`self.M Brake Light`))
  (bind _returnvalue (`KismetMathLibrary.SelectFloat` 2500.0 25.0 (`self.Is Braking`)))
  (if (`KismetSystemLibrary.IsValid` _m_brake_light)
    (`MaterialInstanceDynamic.SetVectorParameterValue` _m_brake_light "Light Color" (struct :`R` 0.035 :`G` 0.000257 :`A` 1.0))
    (`MaterialInstanceDynamic.SetScalarParameterValue` _m_brake_light "Glow Intensity" _returnvalue)
    (`LightComponent.SetIntensity` (`self.Brake Light Left`) _returnvalue)
    (`LightComponent.SetIntensity` (`self.Brake Light Right`) _returnvalue)))

(fn `OnRep_Is Head Light On`
  (bind _head_light_material_slot (`self.Head Light Material Slot`))
  (bind _mesh (`self.Mesh`))
  (if (not (== "None" _head_light_material_slot))
    (`PrimitiveComponent.CreateDynamicMaterialInstance` _mesh (`MeshComponent.GetMaterialIndex` _mesh _head_light_material_slot) (select `bool` (`self.Is Head Light On`) :`false` "/Game/Vehicles/00_Master_Vehicle/Materials/M_Chrome.M_Chrome" :`true` "/Game/Vehicles/00_Master_Vehicle/Materials/Instances/MI_HeadLight.MI_HeadLight" :!type "MaterialInterface Object Reference"))
    (`SceneComponent.SetVisibility` (`self.Head Light Right`) (`self.Is Head Light On`) false)
    (`SceneComponent.SetVisibility` (`self.Head Light Left`) (`self.Is Head Light On`) false)))

(fn `OnRep_Is Reversing`
  (bind _reverse_light_material_slot (`self.Reverse Light Material Slot`))
  (bind _mesh (`self.Mesh`))
  (if (not (== "None" _reverse_light_material_slot))
    (`PrimitiveComponent.CreateDynamicMaterialInstance` _mesh (`MeshComponent.GetMaterialIndex` _mesh _reverse_light_material_slot) (select `bool` (`self.Is Reversing`) :`false` "/Game/Vehicles/00_Master_Vehicle/Materials/M_Chrome.M_Chrome" :`true` "/Game/Vehicles/00_Master_Vehicle/Materials/Instances/MI_ReverseLight_2.MI_ReverseLight_2" :!type "MaterialInterface Object Reference"))))

(fn `OnRep_RPM`)

(fn `PossessPVehicle`
  (params (`New Controller` :type "Controller Object Reference"))
  (returns (`Is Controlled by Player` :type Boolean))
  (bind _engine_sound (`self.Engine Sound`))
  (`AudioComponent.SetSound` _engine_sound "/Game/Vehicles/Camaro/Sounds/Opel/Opel_2_Engine_Cue.Opel_2_Engine_Cue")
  (`AudioComponent.SetBoolParameter` _engine_sound "Engine Started" true)
  (`AudioComponent.Play` _engine_sound 0.0)
  (return (`Controller.IsPlayerController` `New Controller`)))

(fn `Set Steering Angle`
  (params (`Steering Axis` :type "Float (double-precision)"))
  (`/Engine/EditorBlueprintResources/ActorMacros.Switch Has Authority`
    (:`Authority`
      (if (== `Steering Axis` 0.0)
        ;[1 1 1] Steering return to 0
        (set `self.Steering Angle Calc` (`KismetMathLibrary.FInterpTo_Constant` (`self.Steering Angle Calc`) 0.0 (`GameplayStatics.GetWorldDeltaSeconds`) (`self.Steering Fall Speed`)))
        (else
          ;[1 1 1] Steering Rise until limit for each wheel that are set to steer
          (set `self.Steering Angle Calc` (`KismetMathLibrary.FInterpTo_Constant` (`self.Steering Angle Calc`) (* (`self.Max Steer Angle`) `Steering Axis`) (`GameplayStatics.GetWorldDeltaSeconds`) (* (`KismetMathLibrary.Abs` `Steering Axis`) (`CurveFloat.GetFloatValue` (`self.Steering Speed Curve`) (`self.Speed`))))))))))

(fn `Stall Engine`
  (bind _engine_sound (`self.Engine Sound`))
  (set `self.Engine Started` false)
  (set `self.RPM` 0.0)
  (`AudioComponent.SetSound` _engine_sound "/Game/Player/Sounds/0477.0477")
  (`AudioComponent.Play` _engine_sound 0.0))

(fn `Toggle Headlights`
  (set `self.Is Head Light On` (not (`self.Is Head Light On`))))

(fn `Un-Stall Engine`
  (bind _engine_sound (`self.Engine Sound`))
  (`AudioComponent.SetSound` _engine_sound "/Game/Vehicles/Camaro/Sounds/Opel/Opel_2_Engine_Cue.Opel_2_Engine_Cue")
  (`AudioComponent.Play` _engine_sound 0.0))

(fn `UnPossessPVehicle`
  (bind _returnvalue (`SceneComponent.K2_GetComponentToWorld` (`self.Player Location`)))
  (`WheeledVehicleMovementComponent.SetHandbrakeInput` (`self.VehicleMovement`) true)
  (bind _returnvalue_2 (`|SpawnActorFromClass` "/Game/Player/BP_Physic_Pawn.BP_Physic_Pawn_C" (`KismetMathLibrary.MakeTransform` (.location _returnvalue) (`KismetMathLibrary.MakeRotator` 0.0 0.0 (.yaw (.rotation _returnvalue)))) "AdjustIfPossibleButAlwaysSpawn" "OverrideRootScale" null (`self.Is Third Person View`) null))
  (`Controller.Possess` (`self.GetController`) _returnvalue_2)
  (`self.Debug Stats Widget` false)
  (bind _returnvalue_3 (`PrimitiveComponent.GetPhysicsLinearVelocity` (`self.Mesh`) "None"))
  (if (> (`KismetMathLibrary.VSize` _returnvalue_3) 900.0)
    (`/Game/Player/BP_Physic_Pawn.Trigger Ragdoll` _returnvalue_2 (* _returnvalue_3 1.0) "Spine_02"))
  (`AudioComponent.SetBoolParameter` (`self.Engine Sound`) "Engine Started" false)
  (set `self.Engine Started` false))

(fn `Update Vehicle Sounds`
  (locals (`Int Drifting Wheels` :type Integer))
  (bind _tire_sound (`self.Tire Sound`))
  (bind _int_drifting_wheels (`local.Int Drifting Wheels`))
  (for _array_element (`self.Wheels`)
    (if (`.IsDrifting_38_966D437D487EA024956950ABA5F36739` (break `/Game/Vehicles/00_Master_Vehicle/Structs/Wheel_Structure` _array_element))
      (`/Engine/EditorBlueprintResources/StandardMacros.IncrementInt` (`local.Int Drifting Wheels`))))
  (`AudioComponent.AdjustVolume` _tire_sound 0.2 (`KismetMathLibrary.SelectFloat` 1.0 0.0 (> _int_drifting_wheels 0)))
  (`AudioComponent.SetVolumeMultiplier` _tire_sound (/ (`KismetMathLibrary.FClamp` (`KismetMathLibrary.Conv_IntToDouble` _int_drifting_wheels) 1.0 5.0) 2.0))
  (`AudioComponent.SetFloatParameter` (`self.Engine Sound`) "RPM" (`KismetMathLibrary.FClamp` (`WheeledVehicleMovementComponent.GetEngineRotationSpeed` (`self.VehicleMovement`)) (`self.RPM Idle`) (`self.RPM Limit`))))

(fn `UserConstructionScript`)