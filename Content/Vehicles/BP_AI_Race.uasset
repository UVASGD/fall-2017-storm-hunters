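; AI racing controller that possesses a BP_Master_Vehicle and drives it around a looping, index-ordered list of BP_Vehicle_Waypoint actors.
; Each tick it advances waypoints within their acceptable radius, steers by yaw toward the target and prints debug state.
; Desired speed blends from a high default to the target waypoint's speed on approach.
; Throttle and brake are mapped from that speed, with updates skipped while any wheel drifts.
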(event `self.ReceiveBeginPlay`
  (`KismetSystemLibrary.Delay` 0.2)
  (`self.Begin`))

(event `self.ReceiveTick`
  (params (DeltaSeconds :type "Float (single-precision)"))
  (`self.Handle Target Waypoint`)
  (`self.Handle Steering Angle`)
  (`self.Detect Drifting`)
  (`self.Calculate Desired Speed`)
  (`self.Handle Speed`)
  (`self.Print Debug Variables`))

(fn `Begin`
  (bind _waypoint_list (`self.Waypoint List`))
  (bind _asbp_master_vehicle (cast `/Game/Vehicles/00_Master_Vehicle/BP_Master_Vehicle` (`self.K2_GetPawn` self)))
  (`/Game/Vehicles/00_Master_Vehicle/BP_Master_Vehicle.Possess Vehicle` _asbp_master_vehicle self)
  (bind _output_get (set `self.Vehicle` _asbp_master_vehicle))
  (set `/Game/Vehicles/00_Master_Vehicle/BP_Master_Vehicle.Steering Rise Speed` 70.0 _output_get)
  (`SceneComponent.SetVisibility` (`/Game/Vehicles/00_Master_Vehicle/BP_Master_Vehicle.Driver` _output_get) true true)
  (bind _outactors (`GameplayStatics.GetAllActorsOfClass` "/Game/Vehicles/BP_Vehicle_Waypoint.BP_Vehicle_Waypoint_C"))
  (for _array_element _outactors
    (`KismetArrayLibrary.Array_Set` (`self.Waypoint List`) (`/Game/Vehicles/BP_Vehicle_Waypoint.Index` _array_element) _array_element true))
  (set `self.Target Waypoint` (`|GetArrayItem` (`self.Waypoint List`)))
  (set `self.Previous Waypoint` (`|GetArrayItem` _waypoint_list (`KismetArrayLibrary.Array_LastIndex` _waypoint_list)))
  (for _array_element_2 (`/Game/Vehicles/00_Master_Vehicle/BP_Master_Vehicle.Wheels` (`self.Vehicle`))
    (bind (_bonename _radius _steeringangle) (break `/Game/Vehicles/00_Master_Vehicle/Structs/Wheel_Structure` _array_element_2))
    (if (not (== _steeringangle 0.0))
      (`|ExecutionSequence`
        (:`then_0`
          (break))
        (:`then_1`
          (set `self.Maximum Steering` (`KismetMathLibrary.Abs` _steeringangle)))))))

(fn `Calculate Desired Speed`
  (bind _returnvalue (`self.K2_GetActorLocation` (`self.Target Waypoint`)))
  (set `self.Desired Speed` (`KismetMathLibrary.Lerp` 600.0 (`/Game/Vehicles/BP_Vehicle_Waypoint.Desired Speed` (`self.Target Waypoint`)) (`KismetMathLibrary.MapRangeClamped` (`KismetMathLibrary.VSize` (- _returnvalue (`self.K2_GetActorLocation` (`self.Vehicle`)))) 0.0 (`KismetMathLibrary.VSize` (- (`self.K2_GetActorLocation` (`self.Previous Waypoint`)) _returnvalue)) 1.0))))

(fn `Detect Drifting`
  (for _array_element (`/Game/Vehicles/00_Master_Vehicle/BP_Master_Vehicle.Wheels` (`self.Vehicle`))
    (if (`.IsDrifting_38_966D437D487EA024956950ABA5F36739` (break `/Game/Vehicles/00_Master_Vehicle/Structs/Wheel_Structure` _array_element))
      (set `self.Is Drifting` true)
      (break)
      (else
        (set `self.Is Drifting` false)))))

(fn `Handle Speed`
  (bind _desired_speed (`self.Desired Speed`))
  (bind _vehicle (`self.Vehicle`))
  (bind _returnvalue (* (`KismetMathLibrary.VSize` (`self.GetVelocity` _vehicle)) 0.036))
  (bind _returnvalue_2 (`KismetMathLibrary.MapRangeClamped` _returnvalue _desired_speed (+ _desired_speed 20.0) 0.0 1.0))
  (bind _returnvalue_3 (`KismetMathLibrary.MapRangeClamped` _returnvalue 0.0 (`self.Desired Speed`) 1.0))
  (if (`self.Is Drifting`)
    (set `self.Is Accelerating` false)
    (else
      (`/Game/Vehicles/00_Master_Vehicle/BP_Master_Vehicle.Server_Throttle` _vehicle _returnvalue_3)
      (set `self.Is Accelerating` (> _returnvalue_3 0.1))
      (`/Game/Vehicles/00_Master_Vehicle/BP_Master_Vehicle.Server_Brake` (`self.Vehicle`) _returnvalue_2)
      (set `self.Is Braking` (> _returnvalue_2 0.1)))))

(fn `Handle Steering Angle`
  (bind _maximum_steering (`self.Maximum Steering`))
  (bind (_returnvalue_location _returnvalue_rotation) (`KismetMathLibrary.BreakTransform` (`self.GetTransform` (`self.Vehicle`))))
  (bind (_returnvalue_roll _returnvalue_pitch _returnvalue_yaw) (`KismetMathLibrary.BreakRotator` (`KismetMathLibrary.ComposeRotators` (`KismetMathLibrary.NegateRotator` _returnvalue_rotation) (`KismetMathLibrary.FindLookAtRotation` _returnvalue_location (`self.K2_GetActorLocation` (`self.Target Waypoint`))))))
  (set `self.Steering Angle` _returnvalue_yaw)
  (`/Game/Vehicles/00_Master_Vehicle/BP_Master_Vehicle.Server_Steering` (`self.Vehicle`) (`KismetMathLibrary.MapRangeClamped` (`self.Steering Angle`) (* _maximum_steering -1.0) _maximum_steering -1.0 1.0)))

(fn `Handle Target Waypoint`
  (bind _target_waypoint (`self.Target Waypoint`))
  (if (<= (`KismetMathLibrary.VSize` (- (`self.K2_GetActorLocation` (`self.Vehicle`)) (`self.K2_GetActorLocation` _target_waypoint))) (`/Game/Vehicles/BP_Vehicle_Waypoint.Acceptable Radius` _target_waypoint))
    (bind _output_get (set `self.Waypoint Target Index` (select `bool` (== (`KismetArrayLibrary.Array_LastIndex` (`self.Waypoint List`)) (`self.Waypoint Target Index`)) :`false` (+ (`self.Waypoint Target Index`) 1))))
    (set `self.Previous Waypoint` (`self.Target Waypoint`))
    (set `self.Target Waypoint` (`|GetArrayItem` (`self.Waypoint List`) _output_get))))

(fn `Print Debug Variables`
  (`KismetSystemLibrary.PrintString` (`KismetMathLibrary.SelectString` "Accelerating!" "" (`self.Is Accelerating`)) true true (struct :`R` 0.69 :`A` 1.0) 0.0)
  (`KismetSystemLibrary.PrintString` (`KismetMathLibrary.SelectString` "Braking!" "" (`self.Is Braking`)) true true (struct :`R` 0.69 :`A` 1.0) 0.0)
  (`KismetSystemLibrary.PrintString` (`KismetMathLibrary.SelectString` "Drifting!" "" (`self.Is Drifting`)) true true (struct :`R` 0.69 :`A` 1.0) 0.0)
  (`KismetSystemLibrary.PrintString` (`KismetStringLibrary.Concat_StrStr` "Target Waypoint : " (`KismetStringLibrary.Conv_IntToString` (`self.Waypoint Target Index`))) true true (struct :`R` 0.006193 :`G` 0.69 :`A` 1.0) 0.0)
  (`KismetSystemLibrary.PrintString` (`KismetStringLibrary.Concat_StrStr` "Steering Angle : " (`KismetStringLibrary.Conv_IntToString` (`KismetMathLibrary.Round` (`self.Steering Angle`)))) true true (struct :`R` 0.006193 :`G` 0.69 :`A` 1.0) 0.0)
  (`KismetSystemLibrary.PrintString` (`KismetStringLibrary.Concat_StrStr` "Speed (km/h) : " (`KismetStringLibrary.Conv_IntToString` (`KismetMathLibrary.Round` (`/Game/Vehicles/00_Master_Vehicle/BP_Master_Vehicle.Speed` (`self.Vehicle`))))) true true (struct :`R` 0.006193 :`G` 0.69 :`A` 1.0) 0.0))

(fn `UserConstructionScript`)