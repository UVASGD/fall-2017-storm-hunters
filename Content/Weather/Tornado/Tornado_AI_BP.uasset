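; AI controller that drives a tornado pawn around a looping path of waypoints.
; After a short delay it gathers the waypoints matching the pawn's path index and orders them by their own index.
; Each tick it advances the target once within that waypoint's horizontal acceptance radius.
; It steers by easing the inner cylinder's physics X/Y velocity toward the target, using a fixed interpolation step rather than frame delta.
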(event `self.ReceiveBeginPlay`
  (`KismetSystemLibrary.Delay` 0.2)
  (`self.Initialize`))

(event `self.ReceiveTick`
  (params (DeltaSeconds :type "Float (single-precision)"))
  (if (`self.ReadyToStart`)
    (`self.Handle Target Waypoint`)
    (`self.Move to Waypoint`)))

(fn `Handle Target Waypoint`
  (bind _target_waypoint (`self.Target Waypoint`))
  (bind (_returnvalue_x _returnvalue_y) (`KismetMathLibrary.BreakVector` (- (`self.K2_GetActorLocation` (`self.Tornado`)) (`self.K2_GetActorLocation` _target_waypoint))))
  (if (<= (`KismetMathLibrary.VSize2D` (`KismetMathLibrary.MakeVector2D` _returnvalue_x _returnvalue_y)) (`/Game/Weather/Tornado/Tornado_Waypoint_BP.AcceptableRadius` _target_waypoint))
    (bind _output_get (set `self.WaypointTargetIndex` (select `bool` (== (`KismetArrayLibrary.Array_LastIndex` (`self.Waypoint List`)) (`self.WaypointTargetIndex`)) :`false` (+ (`self.WaypointTargetIndex`) 1))))
    (set `self.Previous Waypoint` (`self.Target Waypoint`))
    (set `self.Target Waypoint` (`|GetArrayItem` (`self.Waypoint List`) _output_get))))

(fn `Initialize`
  (bind _waypoint_list (`self.Waypoint List`))
  (bind _astornado_pawn_bp (cast `/Game/Weather/Tornado/Tornado_Pawn_BP` (`self.K2_GetPawn` self)))
  (set `self.Tornado` _astornado_pawn_bp)
  (bind _outactors (`GameplayStatics.GetAllActorsOfClass` "/Game/Weather/Tornado/Tornado_Waypoint_BP.Tornado_Waypoint_BP_C"))
  (for _array_element _outactors
    (if (== (`/Game/Weather/Tornado/Tornado_Waypoint_BP.TornadoIndex` _array_element) (`/Game/Weather/Tornado/Tornado_Pawn_BP.PathIndex` (`self.Tornado`)))
      (`KismetArrayLibrary.Array_Set` (`self.Waypoint List`) (`/Game/Weather/Tornado/Tornado_Waypoint_BP.Index` _array_element) _array_element true)))
  (set `self.Target Waypoint` (`|GetArrayItem` (`self.Waypoint List`)))
  (set `self.Previous Waypoint` (`|GetArrayItem` _waypoint_list (`KismetArrayLibrary.Array_LastIndex` _waypoint_list)))
  (set `self.ReadyToStart` true))

(fn `Move to Waypoint`
  (bind _tornado (`self.Tornado`))
  (bind _inner_cyl (`/Game/Weather/Tornado/Tornado_Pawn_BP.Inner_Cyl` _tornado))
  (bind (_returnvalue_x _returnvalue_y) (`KismetMathLibrary.BreakVector` (* (`KismetMathLibrary.Normal` (- (`self.K2_GetActorLocation` (`self.Target Waypoint`)) (`self.K2_GetActorLocation` _tornado))) (* (`/Game/Weather/Tornado/Tornado_Pawn_BP.BaseLinSpeedFactor` _tornado) 1000.0))))
  (bind _returnvalue (`PrimitiveComponent.GetPhysicsLinearVelocity` _inner_cyl "None"))
  (`PrimitiveComponent.SetPhysicsLinearVelocity` _inner_cyl (`KismetMathLibrary.MakeVector` (`KismetMathLibrary.FInterpTo` (.x _returnvalue) _returnvalue_x 0.001 10.0) (`KismetMathLibrary.FInterpTo` (.y _returnvalue) _returnvalue_y 0.001 10.0)) false "None"))

(fn `UserConstructionScript`)