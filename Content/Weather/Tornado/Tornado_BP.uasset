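; Tornado actor that pulls in, swirls and lifts Mercedes_BP vehicles caught inside it.
; Overlaps with inner and outer cylinders, sized from radius and height in the construction script, sort actors into two zone lists.
; Each Tick applies CalculateForces to vehicle meshes, with stronger spin and lift but weaker pull in the inner zone.
; Forces combine radial, tangential (selectable direction) and vertical components, scaled by base speed and fading linearly toward the outer radius.
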(event `self.Inner_Cyl.OnComponentBeginOverlap`
  (params (OverlappedComponent :type "PrimitiveComponent Object Reference") (OtherActor :type "Actor Object Reference") (OtherComp :type "PrimitiveComponent Object Reference") (OtherBodyIndex :type Integer) (bFromSweep :type Boolean) (SweepResult :type "HitResult Structure (by ref)"))
  (`KismetArrayLibrary.Array_Add` (`self.Inside_Inner`) OtherActor)
  (`KismetArrayLibrary.Array_RemoveItem` (`self.Inside_Outer`) OtherActor))

(event `self.ReceiveTick`
  (params (DeltaSeconds :type "Float (single-precision)"))
  (if (or (> (`KismetArrayLibrary.Array_Length` (`self.Inside_Inner`)) 0) (> (`KismetArrayLibrary.Array_Length` (`self.Inside_Outer`)) 0))
    (for _array_element (`self.Inside_Outer`)
      (bind _asmercedes_bp (cast `/Game/Vehicles/Mercedes/Mercedes_BP` _array_element))
      (bind _returnforce (`self.CalculateForces` (5000000.0 3000000.0 2000000.0) _asmercedes_bp))
      (`PrimitiveComponent.AddForce` (`WheeledVehicle.Mesh` _asmercedes_bp) _returnforce "None" false))
    (for _array_element_2 (`self.Inside_Inner`)
      (bind _asmercedes_bp_2 (cast `/Game/Vehicles/Mercedes/Mercedes_BP` _array_element_2))
      (bind _returnforce_2 (`self.CalculateForces` (1000000.0 5000000.0 8000000.0) _asmercedes_bp_2))
      (`PrimitiveComponent.AddForce` (`WheeledVehicle.Mesh` _asmercedes_bp_2) _returnforce_2 "None" false))))

(event `self.Inner_Cyl.OnComponentEndOverlap`
  (params (OverlappedComponent :type "PrimitiveComponent Object Reference") (OtherActor :type "Actor Object Reference") (OtherComp :type "PrimitiveComponent Object Reference") (OtherBodyIndex :type Integer))
  (`KismetArrayLibrary.Array_RemoveItem` (`self.Inside_Inner`) OtherActor)
  (`KismetArrayLibrary.Array_Add` (`self.Inside_Outer`) OtherActor))

(event `self.Outer_Cyl.OnComponentBeginOverlap`
  (params (OverlappedComponent :type "PrimitiveComponent Object Reference") (OtherActor :type "Actor Object Reference") (OtherComp :type "PrimitiveComponent Object Reference") (OtherBodyIndex :type Integer) (bFromSweep :type Boolean) (SweepResult :type "HitResult Structure (by ref)"))
  (`KismetArrayLibrary.Array_Add` (`self.Inside_Outer`) OtherActor))

(event `self.Outer_Cyl.OnComponentEndOverlap`
  (params (OverlappedComponent :type "PrimitiveComponent Object Reference") (OtherActor :type "Actor Object Reference") (OtherComp :type "PrimitiveComponent Object Reference") (OtherBodyIndex :type Integer))
  (`KismetArrayLibrary.Array_RemoveItem` (`self.Inside_Outer`) OtherActor))

(fn `CalculateForces`
  (params (ForceFactor :type "Vector Structure") (Actor :type "Actor Object Reference"))
  (returns (ReturnForce :type "Vector Structure"))
  (bind _outerradius (`self.OuterRadius`))
  (bind (_returnvalue_x _returnvalue_y) (`KismetMathLibrary.BreakVector` (- (`self.K2_GetActorLocation`) (`self.K2_GetActorLocation` Actor))))
  (bind _returnvalue (`KismetMathLibrary.Normal2D` (`KismetMathLibrary.MakeVector2D` _returnvalue_x _returnvalue_y)))
  (bind (_returnvalue_x_2 _returnvalue_y_2) (`KismetMathLibrary.BreakVector2D` (* (select `bool` (`self.SpinCounterClockwise`) :`false` (-1.0 1.0) :`true` (1.0 -1.0) :!type "Vector2D Structure") _returnvalue)))
  (bind _returnvalue_2 (/ (- _outerradius (`KismetMathLibrary.VSize2D` (`KismetMathLibrary.MakeVector2D` _returnvalue_x _returnvalue_y))) _outerradius))
  (bind (_returnvalue_x_3 _returnvalue_y_3) (`KismetMathLibrary.BreakVector2D` (+ (* (`KismetMathLibrary.MakeVector2D` _returnvalue_y_2 _returnvalue_x_2) (* (* (`self.BaseRotSpeedFactor`) ForceFactor_Y) _returnvalue_2)) (* _returnvalue (* (* (`self.BaseRotSpeedFactor`) ForceFactor_X) _returnvalue_2)))))
  (return (`KismetMathLibrary.MakeVector` _returnvalue_x_3 _returnvalue_y_3 (* (* (`self.BaseRotSpeedFactor`) ForceFactor_Z) _returnvalue_2))))

(fn `UserConstructionScript`
  (bind _returnvalue (/ (`self.InnerRadius`) 50.0))
  (bind _returnvalue_2 (/ (`self.OuterRadius`) 50.0))
  (bind _returnvalue_3 (/ (`self.Height`) 500.0))
  (`SceneComponent.SetWorldScale3D` (`self.Inner_Cyl`) (`KismetMathLibrary.MakeVector` _returnvalue _returnvalue _returnvalue_3))
  (`SceneComponent.SetWorldScale3D` (`self.Outer_Cyl`) (`KismetMathLibrary.MakeVector` _returnvalue_2 _returnvalue_2 _returnvalue_3)))