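; Level manager for a tornado driving game, switching the player between free roam and races and running the car select, race menu and race end widgets.
; CreateRace reads Race_Data_Table to teleport the car, reset debris and spawn checkpoints, a race manager, tornados and waypoints, which PurgeRace destroys.
; Outside races, a looping timer spawns randomly sized, placed and paced tornados with waypoints, all on limited lifespans with cycling path indices.
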(event `self.ReceiveBeginPlay`
  (if (`self.InitialPurge`)
    (`self.PurgeRace`))
  (`self.Initialize`)
  (set `self.ReadyToStart` true)
  (`KismetSystemLibrary.K2_SetTimer` null "SpawnTornado" (`self.FRSpawnTime`) true)
  (set `self.FRSpawnMax` (+ (`KismetMathLibrary.FCeil` (/ (`self.FRLifetime`) (`self.FRSpawnTime`))) 1))
  (`KismetSystemLibrary.Delay` 1.0)
  (`self.ShowSelectCar` true))

(event `self.ReceiveTick`
  (params (DeltaSeconds :type "Float (single-precision)")))

(event `InputAction|Menu_Open`
  (params (Key :type "Key Structure"))
  (:`Pressed`
    (if (not (`/Game/Vehicles/Master_Vehicle/Master_Vehicle_BP.InRace` (`self.Player_Vehicle`)))
      (`self.ShowSelectCar` true)
      (else
        (`self.ShowRaceMenu` true)))))

(event `Key|B`
  (params (Key :type "Key Structure")))

(event `RaceWon`
  (`self.ShowRaceEnd` true true)
  (set `self.RaceEndInputEnabled` true)
  (`KismetSystemLibrary.Delay` 0.1)
  (`GameplayStatics.SetGamePaused` true))

(event `InputAction|Menu_Select` :paused true
  (params (Key :type "Key Structure"))
  (:`Pressed`
    (if (`self.RaceEndInputEnabled`)
      (`self.GoFreeRoam`))))

(event `RaceLost`
  (`self.ShowRaceEnd` true)
  (set `self.RaceEndInputEnabled` true))

(event `InputAction|Menu_Back` :paused true
  (params (Key :type "Key Structure"))
  (:`Pressed`
    (if (`self.RaceEndInputEnabled`)
      (`self.RestartRace`))))

(event `RestartRace`
  (set `self.RaceEndInputEnabled` false)
  (`GameplayStatics.SetGamePaused` false)
  (`self.ShowRaceMenu` false)
  (`self.ShowRaceEnd` false)
  (`self.PurgeRace`)
  (`self.EnableInput` (`self.Player_Vehicle`) null)
  (`self.CreateRace` (`self.TargetRaceName`)))

(event `GoFreeRoam`
  (bind _player_vehicle (`self.Player_Vehicle`))
  (set `self.RaceEndInputEnabled` false)
  (`GameplayStatics.SetGamePaused` false)
  (`self.ShowRaceMenu` false)
  (`self.ShowRaceEnd` false)
  (`self.PurgeRace`)
  (`self.EnableInput` _player_vehicle null)
  (`/Game/Vehicles/Master_Vehicle/Master_Vehicle_BP.Un-Stall Engine` _player_vehicle)
  (set `/Game/Vehicles/Master_Vehicle/Master_Vehicle_BP.Engine Started` true _player_vehicle)
  (`self.ShowRaceEntry` true))

(event `SpawnRaceTornado`
  (params (PathIndex :type Integer))
  (bind (_start_location _inner_radius _outer_radius _height _spin_counterclockwise _base_lin_speed _base_rot_speed _path_index) (break `/Game/Weather/Tornado/Tornado_Setup_Struct` (`|GetArrayItem` (`self.RaceTornados`) PathIndex)))
  (`|SpawnActorFromClass` "/Game/Weather/Tornado/Tornado_Pawn_BP.Tornado_Pawn_BP_C" (`KismetMathLibrary.MakeTransform` _start_location) "Undefined" "OverrideRootScale" null _inner_radius _outer_radius _height _spin_counterclockwise _base_rot_speed _base_lin_speed _path_index null))

(event `DestroyRaceTornado`
  (params (PathIndex :type Integer))
  (bind _outactors (`GameplayStatics.GetAllActorsOfClass` "/Game/Weather/Tornado/Tornado_Pawn_BP.Tornado_Pawn_BP_C"))
  (for _array_element _outactors
    (if (== (`/Game/Weather/Tornado/Tornado_Pawn_BP.PathIndex` _array_element) PathIndex)
      (`self.K2_DestroyActor` _array_element))))

(fn `CreateRace`
  (params (RaceName :type Name))
  (bind _player_vehicle (`self.Player_Vehicle`))
  (bind _mesh (`WheeledVehicle.Mesh` _player_vehicle))
  (if (not (`/Game/Vehicles/Master_Vehicle/Master_Vehicle_BP.InRace` (`self.Player_Vehicle`)))
    (bind _outactors (`GameplayStatics.GetAllActorsOfClass` "/Game/Weather/Tornado/Tornado_Pawn_BP.Tornado_Pawn_BP_C"))
    (for _array_element _outactors
      (`self.K2_DestroyActor` _array_element))
    (bind _outactors_2 (`GameplayStatics.GetAllActorsOfClass` "/Game/Weather/Tornado/Tornado_Waypoint_BP.Tornado_Waypoint_BP_C"))
    (for _array_element_2 _outactors_2
      (`self.K2_DestroyActor` _array_element_2))
    (for _array_element_3 (`self.LevelDebris`)
      (`/Game/Meshes/Debris/Debris_BP.Reset_Location` _array_element_3))
    (for _array_element_4 (`self.LevelSkeletalDebris`)
      (`/Game/Meshes/Debris/Debris_Skeletal_BP.Reset_Location` _array_element_4))
    (bind _returnvalue (`|GetDataTableRow` "/Game/Races/Race_Data_Table.Race_Data_Table" RaceName)
      (:`then`
        (`PrimitiveComponent.SetPhysicsLinearVelocity` _mesh (0.0 0.0 0.0) false "None")
        (`PrimitiveComponent.SetPhysicsAngularVelocity` _mesh (0.0 0.0 0.0) false "None")
        (`self.K2_TeleportTo` _player_vehicle (`.Player_Start_Location_30_B72F933B4C8B8112D667B5A2E0FCC64F` (break `/Game/Races/Race_Struct` _returnvalue)) (`.Player_Start_Rotation_5_93C3563A4941F7A32D4925B8110E20B8` (break `/Game/Races/Race_Struct` _returnvalue)))
        (set `self.TargetRaceName` (break `/Game/Races/Race_Struct` _returnvalue))
        (for (_array_element_5 _array_index) (`.Checkpoints_42_69CD2FCF41F974BBEA63C1BF128D6E64` (break `/Game/Races/Race_Struct` _returnvalue))
          (bind (_location _acceptable_radius _time_to_next _tornado_event_index _spawn_event) (break `/Game/Races/Checkpoint_Setup_Struct` _array_element_5))
          (`|SpawnActorFromClass` "/Game/Races/Race_Checkpoint_BP.Race_Checkpoint_BP_C" (`KismetMathLibrary.MakeTransform` _location) "Undefined" "OverrideRootScale" null _acceptable_radius false _array_index _time_to_next _tornado_event_index _spawn_event null))
        (bind _returnvalue_2 (`|SpawnActorFromClass` "/Game/Races/Race_Manager_BP.Race_Manager_BP_C" (`KismetMathLibrary.MakeTransform` (0.0 0.0 0.0)) "Undefined" "OverrideRootScale" null (`.Race_Start_Time_18_B722B9B64DE9C1B3D5B954BFA0E093CF` (break `/Game/Races/Race_Struct` _returnvalue)) (`.Race_Num_Laps_21_A0FFEE554CC6D6A9310F94822930FA2B` (break `/Game/Races/Race_Struct` _returnvalue)) (`.Use_Timer_41_D1707F074B3599C6459960AAD46D5992` (break `/Game/Races/Race_Struct` _returnvalue)) null))
        (set `self.CurrentRaceMan` _returnvalue_2)
        (for (_array_element_6 _array_index_2) (`.Tornados_44_957FCDFC4845FDCA3AAFE1AD1E917CB7` (break `/Game/Races/Race_Struct` _returnvalue))
          (`KismetArrayLibrary.Array_Set` (`self.RaceTornados`) _array_index_2 _array_element_6 true)
          (bind (_start_location _inner_radius _outer_radius _height _spin_counterclockwise _base_lin_speed _base_rot_speed _path_index _spawn_at_start) (break `/Game/Weather/Tornado/Tornado_Setup_Struct` _array_element_6))
          (if _spawn_at_start
            (`|SpawnActorFromClass` "/Game/Weather/Tornado/Tornado_Pawn_BP.Tornado_Pawn_BP_C" (`KismetMathLibrary.MakeTransform` _start_location) "Undefined" "OverrideRootScale" null _inner_radius _outer_radius _height _spin_counterclockwise _base_rot_speed _base_lin_speed _path_index null)))
        (for _array_element_7 (`.Tornado_WP_34_48F7D44D4B71E2794B31188C148B1A9A` (break `/Game/Races/Race_Struct` _returnvalue))
          (bind (_location_2 _acceptable_radius_2 _index _tornado_index) (break `/Game/Weather/Tornado/Tornado_WP_Setup_Struct` _array_element_7))
          (`|SpawnActorFromClass` "/Game/Weather/Tornado/Tornado_Waypoint_BP.Tornado_Waypoint_BP_C" (`KismetMathLibrary.MakeTransform` _location_2) "Undefined" "OverrideRootScale" null _acceptable_radius_2 _index true _tornado_index null)
          (`self.ShowRaceEntry` false))))))

(fn `Initialize`
  (bind _outactors (`GameplayStatics.GetAllActorsOfClass` "/Game/Vehicles/Master_Vehicle/Master_Vehicle_BP.Master_Vehicle_BP_C"))
  (for _array_element _outactors
    (if (`Pawn.IsPlayerControlled` _array_element)
      (bind _output_get (set `self.Player_Vehicle` _array_element))
      (set `/Game/Vehicles/Master_Vehicle/Master_Vehicle_BP.Engine Started` true _output_get)
      (set `/Game/Vehicles/Master_Vehicle/Master_Vehicle_BP.InRace` false _output_get)
      (bind _outactors_2 (`GameplayStatics.GetAllActorsOfClass` "/Game/Races/Race_Entry_BP.Race_Entry_BP_C"))
      (for (_array_element_2 _array_index) _outactors_2
        (set `/Game/Races/Race_Entry_BP.RaceMaster` self _array_element_2)
        (`KismetArrayLibrary.Array_Set` (`self.RaceEntries`) _array_index _array_element_2 true))
      (bind _outactors_3 (`GameplayStatics.GetAllActorsOfClass` "/Game/Meshes/Debris/Debris_BP.Debris_BP_C"))
      (for (_array_element_3 _array_index_2) _outactors_3
        (`KismetArrayLibrary.Array_Set` (`self.LevelDebris`) _array_index_2 _array_element_3 true))
      (bind _outactors_4 (`GameplayStatics.GetAllActorsOfClass` "/Game/Meshes/Debris/Debris_Skeletal_BP.Debris_Skeletal_BP_C"))
      (for (_array_element_4 _array_index_3) _outactors_4
        (`KismetArrayLibrary.Array_Set` (`self.LevelSkeletalDebris`) _array_index_3 _array_element_4 true))
      (`self.EnableInput` (`GameplayStatics.GetPlayerController` 0)))))

(fn `PurgeRace`
  (bind _outactors (`GameplayStatics.GetAllActorsOfClass` "/Game/Races/Race_Manager_BP.Race_Manager_BP_C"))
  (for _array_element _outactors
    (`self.K2_DestroyActor` _array_element))
  (bind _outactors_2 (`GameplayStatics.GetAllActorsOfClass` "/Game/Races/Race_Checkpoint_BP.Race_Checkpoint_BP_C"))
  (for _array_element_2 _outactors_2
    (`self.K2_DestroyActor` _array_element_2))
  (`KismetArrayLibrary.Array_Clear` (`self.RaceTornados`))
  (bind _outactors_3 (`GameplayStatics.GetAllActorsOfClass` "/Game/Weather/Tornado/Tornado_Pawn_BP.Tornado_Pawn_BP_C"))
  (for _array_element_3 _outactors_3
    (`self.K2_DestroyActor` _array_element_3))
  (bind _outactors_4 (`GameplayStatics.GetAllActorsOfClass` "/Game/Weather/Tornado/Tornado_Waypoint_BP.Tornado_Waypoint_BP_C"))
  (for _array_element_4 _outactors_4
    (`self.K2_DestroyActor` _array_element_4)))

(fn `ShowRaceEnd`
  (params (Show :type Boolean) (RaceWon :type Boolean))
  (bind _raceend (`self.RaceEnd`))
  (bind _player_vehicle (`self.Player_Vehicle`))
  (bind _vehiclemovement (`WheeledVehicle.VehicleMovement` _player_vehicle))
  (if Show
    (`/Engine/EditorBlueprintResources/StandardMacros.IsValid` (`self.RaceEnd`)
      (:`Is Valid`
        _)
      (:`Is Not Valid`
        (bind _returnvalue (`|CreateWidget` "/Game/UMG/Race_End.Race_End_C"))
        (bind _output_get (set `self.RaceEnd` _returnvalue))
        (set `/Game/UMG/Race_End.RaceMaster` self _output_get)
        (`UserWidget.AddToViewport` _output_get 1)))
    (set `/Game/UMG/Race_End.RaceWon` RaceWon _raceend)
    (set `/Game/UMG/Race_End.RaceName` (`self.TargetRaceName`) _raceend)
    (`/Game/UMG/Race_End.SetTexts` _raceend)
    (`Widget.SetVisibility` _raceend "Visible")
    (`WheeledVehicleMovementComponent.SetThrottleInput` _vehiclemovement 0.0)
    (`WheeledVehicleMovementComponent.SetSteeringInput` _vehiclemovement 0.0)
    (`WheeledVehicleMovementComponent.SetBrakeInput` _vehiclemovement 1.0)
    (`self.DisableInput` _player_vehicle null)
    (else
      (`Widget.SetVisibility` (`self.RaceEnd`) "Collapsed"))))

(fn `ShowRaceEntry`
  (params (Show :type Boolean))
  (if Show
    (for _array_element (`self.RaceEntries`)
      (`self.SetActorHiddenInGame` _array_element false)
      (set `/Game/Races/Race_Entry_BP.IsHidden` false _array_element))
    (else
      (for _array_element_2 (`self.RaceEntries`)
        (`self.SetActorHiddenInGame` _array_element_2 true)
        (set `/Game/Races/Race_Entry_BP.IsHidden` true _array_element_2)))))

(fn `ShowRaceMenu`
  (params (Show :type Boolean))
  (bind _returnvalue (`GameplayStatics.GetPlayerController` 0))
  (bind _returnvalue_2 (`GameplayStatics.GetPlayerController` 0))
  (bind _racemenu (`self.RaceMenu`))
  (if Show
    (`/Engine/EditorBlueprintResources/StandardMacros.IsValid` (`self.RaceMenu`)
      (:`Is Valid`
        _)
      (:`Is Not Valid`
        (bind _returnvalue_3 (`|CreateWidget` "/Game/UMG/Race_Menu.Race_Menu_C"))
        (bind _output_get (set `self.RaceMenu` _returnvalue_3))
        (set `/Game/UMG/Race_Menu.RaceMaster` self _output_get)
        (set `/Game/UMG/Race_Menu.TargetVehicle` (`self.Player_Vehicle`) _returnvalue_3)
        (`UserWidget.AddToViewport` _returnvalue_3 3)))
    (`Widget.SetVisibility` _racemenu "Visible")
    (set `PlayerController.bShowMouseCursor` true _returnvalue)
    (`WidgetBlueprintLibrary.SetInputMode_GameAndUIEx` _returnvalue _racemenu)
    (`GameplayStatics.SetGamePaused` true)
    (set `self.RaceEndInputEnabled` true)
    (else
      (`Widget.SetVisibility` (`self.RaceMenu`) "Collapsed")
      (set `PlayerController.bShowMouseCursor` false _returnvalue_2)
      (`WidgetBlueprintLibrary.SetInputMode_GameOnly` _returnvalue_2)
      (set `self.RaceEndInputEnabled` false))))

(fn `ShowSelectCar`
  (params (Show :type Boolean))
  (bind _returnvalue (`GameplayStatics.GetPlayerController` 0))
  (bind _returnvalue_2 (`GameplayStatics.GetPlayerController` 0))
  (if Show
    (`/Engine/EditorBlueprintResources/StandardMacros.IsValid` (`self.CarSelect`)
      (:`Is Valid`
        _)
      (:`Is Not Valid`
        (bind _returnvalue_3 (`|CreateWidget` "/Game/UMG/Car_Select.Car_Select_C"))
        (bind _output_get (set `self.CarSelect` _returnvalue_3))
        (set `/Game/UMG/Car_Select.RaceMaster` self _returnvalue_3)
        (set `/Game/UMG/Car_Select.TargetVehicle` (`self.Player_Vehicle`) _returnvalue_3)
        (`UserWidget.AddToViewport` _output_get 2)))
    (`Widget.SetVisibility` (`self.CarSelect`) "Visible")
    (set `PlayerController.bShowMouseCursor` true _returnvalue_2)
    (`WidgetBlueprintLibrary.SetInputMode_GameAndUIEx` _returnvalue_2 _returnvalue_3)
    (`GameplayStatics.SetGamePaused` true)
    (else
      (`Widget.SetVisibility` (`self.CarSelect`) "Collapsed")
      (set `PlayerController.bShowMouseCursor` false _returnvalue)
      (`WidgetBlueprintLibrary.SetInputMode_GameOnly` _returnvalue))))

(fn `SpawnTornado`
  (locals (NewTIndex :type Integer :default 0) (TornadoStrength :type "Float (double-precision)" :default 0.0))
  (bind _frspawncurrent (`self.FRSpawnCurrent`))
  (bind _tornadostrength (`local.TornadoStrength`))
  (bind _newtindex (`local.NewTIndex`))
  (bind _returnvalue (+ (`self.FRLifetime`) 5.0))
  (if (not (`/Game/Vehicles/Master_Vehicle/Master_Vehicle_BP.InRace` (`self.Player_Vehicle`)))
    (if (== _frspawncurrent (`self.FRSpawnMax`))
      (bind _output_get (set `local.NewTIndex` 0))
      (set `self.FRSpawnCurrent` _output_get)
      (else
        (bind _output_get_2 (set `local.NewTIndex` (+ _frspawncurrent 1)))
        (set `self.FRSpawnCurrent` _output_get_2)))
    (bind _returnvalue_2 (`|SpawnActorFromClass` "/Game/Weather/Tornado/Tornado_Waypoint_BP.Tornado_Waypoint_BP_C" (`KismetMathLibrary.MakeTransform` (`KismetMathLibrary.MakeVector` (`KismetMathLibrary.RandomFloatInRange` -372000.0 426000.0) (`KismetMathLibrary.RandomFloatInRange` -372000.0 426000.0) -11000.0)) "Undefined" "OverrideRootScale" null 1500.0 0 true _newtindex null))
    (`self.SetLifeSpan` _returnvalue_2 _returnvalue)
    (bind _returnvalue_3 (`|SpawnActorFromClass` "/Game/Weather/Tornado/Tornado_Waypoint_BP.Tornado_Waypoint_BP_C" (`KismetMathLibrary.MakeTransform` (`KismetMathLibrary.MakeVector` (`KismetMathLibrary.RandomFloatInRange` -372000.0 426000.0) (`KismetMathLibrary.RandomFloatInRange` -372000.0 426000.0) -11000.0)) "Undefined" "OverrideRootScale" null 1500.0 1 true (`local.NewTIndex`) null))
    (`self.SetLifeSpan` _returnvalue_3 _returnvalue)
    (set `local.TornadoStrength` (* (`KismetMathLibrary.RandomFloatInRange` 2500.0 2700.0) (`KismetMathLibrary.Exp` (`KismetMathLibrary.RandomFloatInRange` 0.0 3.0))))
    (bind _returnvalue_4 (`|SpawnActorFromClass` "/Game/Weather/Tornado/Tornado_Pawn_BP.Tornado_Pawn_BP_C" (`KismetMathLibrary.MakeTransform` (`KismetMathLibrary.MakeVector` (`KismetMathLibrary.RandomFloatInRange` -372000.0 426000.0) (`KismetMathLibrary.RandomFloatInRange` -372000.0 426000.0))) "Undefined" "OverrideRootScale" null _tornadostrength (* _tornadostrength (`KismetMathLibrary.RandomFloatInRange` 2.5 4.0)) 200000.0 (`KismetMathLibrary.RandomBool`) (`KismetMathLibrary.FClamp` (/ (`KismetMathLibrary.Loge` (/ _tornadostrength 2600.0)) 2.0) 0.6 1.2) (`KismetMathLibrary.RandomFloatInRange` 0.5 6.0) _newtindex null))
    (`self.SetLifeSpan` _returnvalue_4 (`self.FRLifetime`))))

(fn `UserConstructionScript`)