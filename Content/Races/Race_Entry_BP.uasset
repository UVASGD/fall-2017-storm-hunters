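; Race entry point actor that lets the player start a named race by driving into its zone.
; Overlap by the Mercedes_BP on the cylinder enables player input on the actor, and leaving disables it.
; While enabled and not hidden, pressing Menu_Select asks RaceMaster to create the race by name.
; The construction script sizes the cylinder from AcceptableRadius and sets the race name text.
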(event `self.ReceiveActorBeginOverlap`
  (params (OtherActor :type "Actor Object Reference")))

(event `self.Cylinder.OnComponentBeginOverlap`
  (params (OverlappedComponent :type "PrimitiveComponent Object Reference") (OtherActor :type "Actor Object Reference") (OtherComp :type "PrimitiveComponent Object Reference") (OtherBodyIndex :type Integer) (bFromSweep :type Boolean) (SweepResult :type "HitResult Structure (by ref)"))
  (cast `/Game/Vehicles/Mercedes/Mercedes_BP` OtherActor)
  (`self.EnableInput` (`GameplayStatics.GetPlayerController` 0)))

(event `self.Cylinder.OnComponentEndOverlap`
  (params (OverlappedComponent :type "PrimitiveComponent Object Reference") (OtherActor :type "Actor Object Reference") (OtherComp :type "PrimitiveComponent Object Reference") (OtherBodyIndex :type Integer))
  (cast `/Game/Vehicles/Mercedes/Mercedes_BP` OtherActor)
  (`self.DisableInput` (`GameplayStatics.GetPlayerController` 0)))

(event `InputAction|Menu_Select`
  (params (Key :type "Key Structure"))
  (:`Pressed`
    (if (not (`self.IsHidden`))
      (`/Game/Races/Race_Master_BP.CreateRace` (`self.RaceMaster`) (`self.RaceName`)))))

(fn `UserConstructionScript`
  (bind _returnvalue (/ (`self.AcceptableRadius`) 50.0))
  (`SceneComponent.SetWorldScale3D` (`self.Cylinder`) (`KismetMathLibrary.MakeVector` _returnvalue _returnvalue 20.0))
  (`TextRenderComponent.K2_SetText` (`self.Race_Name`) (`KismetTextLibrary.Conv_NameToText` (`self.RaceName`))))