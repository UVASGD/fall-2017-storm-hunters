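; Race checkpoint actor that sets a car's respawn point during a race.
; When a Mercedes_BP overlaps it, the checkpoint writes its own location to that car's RespawnPos.
; The construction script sizes a tall cylinder from AcceptableRadius, labels it with the checkpoint Index, and applies the HiddenInGame setting to both.
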(event `self.ReceiveActorBeginOverlap`
  (params (OtherActor :type "Actor Object Reference"))
  (bind _asmercedes_bp (cast `/Game/Vehicles/Mercedes/Mercedes_BP` OtherActor))
  (set `/Game/Vehicles/Mercedes/Mercedes_BP.Respawn_Pos` (`self.K2_GetActorLocation`) _asmercedes_bp))

(fn `UserConstructionScript`
  (bind _index_text (`self.Index_Text`))
  (bind _returnvalue (/ (`self.AcceptableRadius`) 50.0))
  (`SceneComponent.SetWorldScale3D` (`self.Cylinder`) (`KismetMathLibrary.MakeVector` _returnvalue _returnvalue 20.0))
  (`SceneComponent.SetHiddenInGame` (`self.Cylinder`) (`self.Hidden_in_Game`) false)
  (`TextRenderComponent.K2_SetText` _index_text (`KismetTextLibrary.Conv_IntToText` (`self.Index`)))
  (`SceneComponent.SetHiddenInGame` _index_text (`self.Hidden_in_Game`) false))