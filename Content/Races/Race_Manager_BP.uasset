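; Race manager actor that runs a timed checkpoint race for the player-controlled Mercedes_BP car.
; On start it orders Race_Checkpoint_BP actors by Index, plays a countdown, then adds the Race_Timer widget and starts the car.
; Tick checks 2D distance to the target checkpoint, adding bonus time and advancing on arrival.
; Wrapping past the last checkpoint wins; running out of time stalls the engine and fails the race.
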(event `self.ReceiveBeginPlay`
  (bind _player (`self.Player`))
  (`KismetSystemLibrary.Delay` 0.2)
  (`self.Initialize`)
  (`KismetSystemLibrary.Delay` 4.0)
  (`GameplayStatics.PlaySound2D` "/Game/Audio/Checkpoint_1.Checkpoint_1")
  (bind _returnvalue (`|CreateWidget` "/Game/UMG/Race_Timer.Race_Timer_C"))
  (bind _output_get (set `self.RaceTimer` _returnvalue))
  (set `/Game/UMG/Race_Timer.TargetRaceManager` self _returnvalue)
  (`UserWidget.AddToViewport` _output_get 2)
  (set `/Game/Vehicles/Mercedes/Mercedes_BP.Engine Started` true _player)
  (set `/Game/Vehicles/Mercedes/Mercedes_BP.RaceStarted` true _player)
  (set `self.ReadyToStart` true))

(event `self.ReceiveTick`
  (params (DeltaSeconds :type "Float (single-precision)"))
  (if (`self.ReadyToStart`)
    (`self.HandleTargetCheckpoint`)
    (if (not (`self.RaceWonB`))
      (`self.UpdateTimer` DeltaSeconds))))

(event `Race Failed`
  (`Widget.RemoveFromParent` (`self.RaceTimer`))
  (set `self.RaceFailedB` true)
  (`/Game/Vehicles/Mercedes/Mercedes_BP.Stall Engine` (`self.Player`))
  (`GameplayStatics.PlaySound2D` "/Game/Audio/Race_Fail.Race_Fail"))

(event `Race Won`
  (set `self.RaceWonB` true)
  (`GameplayStatics.PlaySound2D` "/Game/Audio/Race_Win.Race_Win"))

(fn `HandleTargetCheckpoint`
  (bind _targetcheckpoint (`self.TargetCheckpoint`))
  (bind (_returnvalue_x _returnvalue_y) (`KismetMathLibrary.BreakVector` (- (`self.K2_GetActorLocation` (`self.Player`)) (`self.K2_GetActorLocation` _targetcheckpoint))))
  (if (<= (`KismetMathLibrary.VSize2D` (`KismetMathLibrary.MakeVector2D` _returnvalue_x _returnvalue_y)) (`/Game/Races/Race_Checkpoint_BP.AcceptableRadius` _targetcheckpoint))
    (`GameplayStatics.PlaySound2D` "/Game/Audio/Checkpoint_1.Checkpoint_1")
    (set `self.TimeLeft` (+ (`/Game/Races/Race_Checkpoint_BP.Time_to_Next` (`self.TargetCheckpoint`)) (`self.TimeLeft`)))
    (bind _output_get (set `self.CheckpointTargetIndex` (select `bool` (== (`KismetArrayLibrary.Array_LastIndex` (`self.Checkpoint_List`)) (`self.CheckpointTargetIndex`)) :`false` (+ (`self.CheckpointTargetIndex`) 1))))
    (set `self.PreviousCheckpoint` (`self.TargetCheckpoint`))
    (set `self.TargetCheckpoint` (`|GetArrayItem` (`self.Checkpoint_List`) _output_get))
    (if (== 0 (`self.CheckpointTargetIndex`))
      (`self.Race Won`))))

(fn `Initialize`
  (bind _checkpoint_list (`self.Checkpoint_List`))
  (bind _outactors (`GameplayStatics.GetAllActorsOfClass` "/Game/Vehicles/Mercedes/Mercedes_BP.Mercedes_BP_C"))
  (for _array_element _outactors
    (if (`Pawn.IsPlayerControlled` _array_element)
      (bind _output_get (set `self.Player` _array_element))
      (set `/Game/Vehicles/Mercedes/Mercedes_BP.Engine Started` false _output_get)
      (set `/Game/Vehicles/Mercedes/Mercedes_BP.InRace` true _output_get)))
  (bind _outactors_2 (`GameplayStatics.GetAllActorsOfClass` "/Game/Races/Race_Checkpoint_BP.Race_Checkpoint_BP_C"))
  (for _array_element_2 _outactors_2
    (`KismetArrayLibrary.Array_Set` (`self.Checkpoint_List`) (`/Game/Races/Race_Checkpoint_BP.Index` _array_element_2) _array_element_2 true))
  (set `self.TargetCheckpoint` (`|GetArrayItem` _checkpoint_list))
  (set `self.PreviousCheckpoint` (`|GetArrayItem` _checkpoint_list (`KismetArrayLibrary.Array_LastIndex` _checkpoint_list)))
  (set `self.TimeLeft` (`self.StartingTime`))
  (`GameplayStatics.PlaySound2D` "/Game/Audio/Countdown.Countdown"))

(fn `UpdateTimer`
  (params (DeltaTime :type "Float (double-precision)"))
  (bind _output_get (set `self.TimeLeft` (- (`self.TimeLeft`) DeltaTime)))
  (if (< _output_get 0.0)
    (`self.Race Failed`)
    (set `self.ReadyToStart` false)))

(fn `UserConstructionScript`)