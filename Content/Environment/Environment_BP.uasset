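; Environment actor that sets time-of-day lighting and sky from a StartTime value, using a sun light, sky light and sky sphere.
; The construction script creates a dynamic cloud-sky material, applies cloud, star and sun settings, then calls SetTime.
; SetTime samples the Time_Flow timeline at StartTime to drive sun rotation, light intensities and sky colors, then recaptures the sky light.
; BeginPlay zeroes the timeline play rate, and OnRep_Time is empty.
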(event `self.ReceiveBeginPlay`
  (`TimelineComponent.SetPlayRate` (`self.Time_Flow`) 0.0))

(event `Set Time`
  (bind _returnvalue (`KismetMathLibrary.MapRangeUnclamped` (.pitch (`SceneComponent.K2_GetComponentRotation` (`self.Sun_Light`))) 0.0 -90.0 0.0 1.0))
  (`|ExecutionSequence`
    (:`then_0`
      (bind (_direction _sun_light_pitch _sun_light_yaw _sky_light_intensity _sun_light_intensity _cloud_opacity _horizon_falloff _timeofday _horizon_color _zenith_color _cloud_color) (`Timeline|Time_Flow` :`NewTime` (`self.Start Time`) :!via `SetNewTime`)))
    (:`then_1`
      (`SceneComponent.K2_SetWorldRotation` (`self.Sun_Light`) (`KismetMathLibrary.MakeRotator` 0.0 _sun_light_pitch _sun_light_yaw) false false)
      (`SkyLightComponent.SetIntensity` (`self.Sky_Light`) _sky_light_intensity)
      (`LightComponent.SetIntensity` (`self.Sun_Light`) _sun_light_intensity)
      (`MaterialInstanceDynamic.SetScalarParameterValue` (`self.Sky material`) "Cloud Opacity" _cloud_opacity)
      (`MaterialInstanceDynamic.SetScalarParameterValue` (`self.Sky material`) "Horizon falloff" _horizon_falloff)
      (set `self.Time` _timeofday)
      (`MaterialInstanceDynamic.SetVectorParameterValue` (`self.Sky material`) "Horizon color" _horizon_color)
      (`LightComponent.SetLightColor` (`self.Sun_Light`) _horizon_color true)
      (`MaterialInstanceDynamic.SetVectorParameterValue` (`self.Sky material`) "Zenith color" _zenith_color)
      (`MaterialInstanceDynamic.SetVectorParameterValue` (`self.Sky material`) "Overall color" _cloud_color)
      (`MaterialInstanceDynamic.SetVectorParameterValue` (`self.Sky material`) "Cloud color" _cloud_color)
      (`MaterialInstanceDynamic.SetVectorParameterValue` (`self.Sky material`) "Light direction" (`KismetMathLibrary.Conv_VectorToLinearColor` (`KismetMathLibrary.Conv_RotatorToVector` (`SceneComponent.K2_GetComponentRotation` (`self.Sun_Light`)))))
      (`MaterialInstanceDynamic.SetScalarParameterValue` (`self.Sky material`) "Sun height" (`KismetMathLibrary.SelectFloat` (`KismetMathLibrary.Abs` _returnvalue) 0.0 (< _returnvalue 0.0)))
      (`MaterialInstanceDynamic.SetVectorParameterValue` (`self.Sky material`) "Sun color" (`LightComponentBase.GetLightColor` (`self.Sun_Light`)))
      (`SkyLightComponent.RecaptureSky` (`self.Sky_Light`)))))

(fn `OnRep_Time`)

(fn `UserConstructionScript`
  (bind _returnvalue (`PrimitiveComponent.CreateDynamicMaterialInstance` (`self.Sky Sphere mesh`) 0 "/Engine/EngineSky/M_Sky_Panning_Clouds2.M_Sky_Panning_Clouds2"))
  (set `self.Sky material` _returnvalue)
  (`MaterialInstanceDynamic.SetScalarParameterValue` (`self.Sky material`) "Cloud speed" (`self.Cloud speed`))
  (`MaterialInstanceDynamic.SetScalarParameterValue` (`self.Sky material`) "Stars Brightness" (`self.Stars brightness`))
  (`MaterialInstanceDynamic.SetScalarParameterValue` (`self.Sky material`) "Sun brightness" (`self.Sun brightness`))
  (`self.Set Time`))