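; Skeletal debris Blueprint that keeps its object within world-space bounds.
; On BeginPlay it stores the object's starting transform and starts a looping one-second timer for CheckLocation, avoiding Tick.
; CheckLocation compares the object's position against MinVec and MaxVec on each axis and calls a location reset when outside.
; The Reset_Location event teleports the object back to its starting location and rotation.
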(event `self.ReceiveBeginPlay`
  (set `self.StartTransform` (`SceneComponent.K2_GetComponentToWorld` (`self.Object`)))
  (`KismetSystemLibrary.K2_SetTimer` self "CheckLocation" 1.0 true))

(event `Reset_Location`
  (bind (_starttransform_location _starttransform_rotation) (`KismetMathLibrary.BreakTransform` (`self.StartTransform`)))
  (`SceneComponent.K2_SetWorldLocationAndRotation` (`self.Object`) _starttransform_location _starttransform_rotation false true))

(fn `CheckLocation`
  (bind (_min_vec_x _min_vec_y _min_vec_z) (`KismetMathLibrary.BreakVector` (`self.Min_Vec`)))
  (bind (_max_vec_x _max_vec_y _max_vec_z) (`KismetMathLibrary.BreakVector` (`self.Max_Vec`)))
  (bind (_returnvalue_x _returnvalue_y _returnvalue_z) (`KismetMathLibrary.BreakVector` (`SceneComponent.K2_GetComponentLocation` (`self.Object`))))
  (if (or (> _returnvalue_x _max_vec_x) (> _returnvalue_y _max_vec_y) (> _returnvalue_z _max_vec_z) (< _returnvalue_x _min_vec_x) (< _returnvalue_y _min_vec_y) (< _returnvalue_z _min_vec_z))
    (`self.Reset_Location`)))

(fn `UserConstructionScript`)