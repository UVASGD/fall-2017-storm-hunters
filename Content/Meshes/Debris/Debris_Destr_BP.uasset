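; Destructible debris actor that respawns after being fractured and is kept within set world bounds.
; On fracture it flags itself, waits a fixed delay, spawns a fresh copy at the saved start transform and destroys itself.
; A looping timer checks the component's location against min and max vectors, calling a location reset when outside.
; The reset event teleports unfractured debris back to its start transform.
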(event `RespawnMe`
  (params (HitPoint :type "Vector Structure (by ref)") (HitDirection :type "Vector Structure (by ref)"))
  (set `self.IsFractured` true)
  (`KismetSystemLibrary.Delay` 30.0)
  (bind _returnvalue (`|SpawnActorFromClass` "Debris_Destr_BP_C" (`self.Start_Transform`) "Undefined" "OverrideRootScale" null null))
  (set `/Game/Meshes/Debris/Debris_Destr_BP.Destructible` (`self.Destructible`) _returnvalue)
  (`self.K2_DestroyActor`))

(event `self.ReceiveBeginPlay`
  (add `DestructibleComponent.OnComponentFracture` (`self.Destructible`) (delegate `RespawnMe`))
  (set `self.Start_Transform` (`SceneComponent.K2_GetComponentToWorld` (`self.Destructible`)))
  (`KismetSystemLibrary.K2_SetTimer` self "CheckLocation" 1.0 true))

(event `self.ReceiveTick`
  (params (DeltaSeconds :type "Float (single-precision)")))

(event `Reset_Location`
  (bind (_start_transform_location _start_transform_rotation) (`KismetMathLibrary.BreakTransform` (`self.Start_Transform`)))
  (if (not (`self.IsFractured`))
    (`SceneComponent.K2_SetWorldLocationAndRotation` (`self.Destructible`) _start_transform_location _start_transform_rotation false true)))

(fn `CheckLocation`
  (bind (_min_vec_x _min_vec_y _min_vec_z) (`KismetMathLibrary.BreakVector` (`self.Min_Vec`)))
  (bind (_max_vec_x _max_vec_y _max_vec_z) (`KismetMathLibrary.BreakVector` (`self.Max_Vec`)))
  (bind (_returnvalue_x _returnvalue_y _returnvalue_z) (`KismetMathLibrary.BreakVector` (`SceneComponent.K2_GetComponentLocation` (`self.Destructible`))))
  (if (or (> _returnvalue_x _max_vec_x) (> _returnvalue_y _max_vec_y) (> _returnvalue_z _max_vec_z) (< _returnvalue_x _min_vec_x) (< _returnvalue_y _min_vec_y) (< _returnvalue_z _min_vec_z))
    (`self.Reset_Location`)))

(fn `UserConstructionScript`)